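; BubbleSpace is an actor that fills a spherical shell with randomly placed Bubble actors when play begins.
; It spawns a configurable number of bubbles at random directions and distances between a minimum and maximum radius, then attaches each to its root component.
; Each bubble is also added to the AllSpheres list on the gameInst_VR game instance, making it a shared registry.
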(event EventBeginPlay
  ;[1 1 1] How Many Spheres to make?
  (for _index (range 0 (Variables|Default|GetNumberOfBubbles))
    ;[1 1 1] Create Sphere
    (bind _returnvalue (Game|SpawnActorfromClass "/Game/Blueprints/Bubble.Bubble_C" (Math|Conversions|ToTransform(Vector) (* (Math|Random|RandomUnitVector) (Math|Random|RandomFloatinRange (Variables|Default|GetminRadius) (Variables|Default|GetmaxRadius)))) false 0 0))
    (Class|Actor|AttachRootComponentto _returnvalue (Variables|Default|GetDefaultSceneRoot) "None" "KeepRelativeOffset" true)
    ;[1 1 1] Add to List of All Spheres
    (bind _asgame_inst_vr (Utilities|Casting|CastTogameInst_VR (Game|GetGameInstance)))
    (Utilities|Array|Add (Variables|/Game/Blueprints/gameInst_VR.gameInst_VR_C|GetAll_Spheres _asgame_inst_vr) _returnvalue)))

(event Collision|EventActorBeginOverlap
  (params (OtherActor :type Actor%20Object%20Reference)))

(event EventTick
  (params (DeltaSeconds :type Float%20%28single-precision%29)))

(fn ConstructionScript)