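; BP_Rhombus is a colored bubble-material floor tile that is either solid or a fake the player falls through.
; The construction script applies BubbleColor through a dynamic material and places a trigger box above the cube.
; At BeginPlay, it compares its RGB channels against the GameInstance's SafeColor flags to set IsFake.
; When the player overlaps a fake tile's box, the cube's collision is disabled.
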(event OnComponentBeginOverlap(CollisionBox)
  (params (OtherActor :type Actor%20Object%20Reference) (OtherComp :type Primitive%20Component%20Object%20Reference) (OtherBodyIndex :type Integer) (bFromSweep :type Boolean) (SweepResult :type Hit%20Result%20Structure%20%28by%20ref%29))
  ;[1 1 1] Vanish Fake Floors
  (if (and (Variables|GamePlay|GetisFake) (== OtherActor (Game|GetPlayerCharacter 0)))
    (Collision|SetCollisionEnabled (Variables|Default|GetCube) "NoCollision")))

(event EventBeginPlay
  (bind _bubblecolor (Variables|Modification|GetBubbleColor))
  (bind (_x _y _z) (Math|Vector|BreakVector _bubblecolor))
  ;[1 1 1] Set Fake Floor
  (bind _asgame_instance_library_vr (Utilities|Casting|CastToGameInstance_LibraryVR (Game|GetGameInstance)))
  (bind (_array_element _array_index) (Utilities|Array|ForEachLoopwithBreak (Variables|/Game/LibraryVR/Blueprints/GameInstance_LibraryVR.GameInstance_LibraryVR_C|GetSafeColor _asgame_instance_library_vr))
    (:LoopBody
      (if _array_element
        (Variables|GamePlay|SettmpBool (and (and _array_element (Utilities|Array|Get(acopy) (Utilities|Array|MakeArray (> _x 0.0) (> _y 0.0) (> _z 0.0)) _array_index)) (Variables|GamePlay|GettmpBool)))))
    (:Completed
      (Variables|GamePlay|SetisFake (not (Variables|GamePlay|GettmpBool))))))

(event EventActorBeginOverlap
  (params (OtherActor :type Actor%20Object%20Reference)))

(event EventTick
  (params (DeltaSeconds :type Float%20%28single-precision%29)))

(fn ConstructionScript
  (bind _cube (Variables|Default|GetCube))
  (bind _returnvalue (Transformation|GetWorldLocation _cube))
  (bind (_x _y _z) (Math|Vector|BreakVector _returnvalue))
  (bind _returnvalue_2 (Rendering|Material|CreateDynamicMaterialInstance 0 "/Game/LibraryVR/MaterialInstances/mat_bp0_bubbles_Inst.mat_bp0_bubbles_Inst" :!class /Script/Engine.PrimitiveComponent))
  (bind _output_get (Variables|Default|SetBubbleDynamicMat _returnvalue_2))
  (Rendering|Material|GetBaseMaterial _output_get)
  (Rendering|Material|SetVectorParameterValue (Variables|Default|GetBubbleDynamicMat) "BubbleColor" (Math|Conversions|ToLinearColor(Vector) (Variables|Modification|GetBubbleColor)) :!class /Script/Engine.MaterialInstanceDynamic)
  (Transformation|SetWorldTransform (Variables|Default|GetCollisionBox) (Math|Transform|MakeTransform (Math|Vector|MakeVector _x _y (+ _z 5e+01)) (Transformation|GetWorldRotation _cube) (Transformation|GetWorldScale _cube)) (not (Variables|GamePlay|GettmpBool))))